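; Celestial body actor that traces its predicted trajectory as a spline.
; BeginPlay caches itself cast to CelestialBody, and Tick rebuilds TrajectorySpline every frame from that body's PredictedTrajectory points in world space.
; A ParticleMovement timeline meant to slide a particle system along the spline by normalized distance is present but never runs.
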(event EventBeginPlay
  (bind _ascelestial_body (Utilities|Casting|CastToCelestialBody self))
  (Variables|Default|SetCelestialBody _ascelestial_body))

(event Collision|EventActorBeginOverlap
  (params (OtherActor :type Actor%20Object%20Reference)))

(event EventTick
  (params (DeltaSeconds :type Float%20%28single-precision%29))
  ;[1 1 1] Update trajectory spline
  (Spline|SetSplinePoints (Variables|Default|GetTrajectorySpline) (Variables|/Script/SolarSystem.CelestialBody|GetPredictedTrajectory (Variables|Default|GetCelestialBody)) "World" true))

(fn ConstructionScript)